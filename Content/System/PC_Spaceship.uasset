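; Player controller for a spaceship game that handles the switch to the game over screen.
; Its gameOver event adds the HUD_GameOver widget to the viewport, shows the mouse cursor, disables the player character's input and sets UI-only input focused on that widget.
; A disconnected chain that would create HUD_Menu and set game-only input never runs, and BeginPlay is empty.
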(event Custom|gameOver
  (bind _self self)
  (bind _returnvalue (UserInterface|CreateWidget "/Game/HUD/HUD_GameOver.HUD_GameOver_C" self))
  (UserInterface|Viewport|AddtoViewport _returnvalue 0)
  (Variables|Default|SetbShowMouseCursor true)
  (Input|DisableInput (Game|GetPlayerCharacter 0) _self)
  (Input|SetInputModeUIOnly _self _returnvalue "DoNotLock" false))

(event EventBeginPlay)

(fn ConstructionScript)