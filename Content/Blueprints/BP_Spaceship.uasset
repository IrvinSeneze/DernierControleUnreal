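; Player-controlled spaceship that moves and fires lasers through Enhanced Input.
; BeginPlay adds the spaceship mapping context, and move input drives movement along forward and right vectors derived from control yaw.
; Fire input spawns BP_Laser at the projectile spawn point, then clears CanShoot until the Reload event restores it after ShootDelay.
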(event Custom|Reload
  ;[1 1 1] Permet d'autoriser le vaisseau à retirer
  (Utilities|FlowControl|Delay (Variables|Default|GetShootDelay))
  (Variables|Default|SetcanShoot true))

(event Input|EnhancedActionEvents|EnhancedInputActionINP_Move
  (params (ActionValue :type Vector%202D%20Structure) (ElapsedSeconds :type Float%20%28double-precision%29) (TriggeredSeconds :type Float%20%28double-precision%29) (InputAction :type Input%20Action%20Object%20Reference :default "/Game/System/Inputs/INP_Move.INP_Move"))
  (bind _returnvalue (Pawn|GetControlRotation :!class /Script/Engine.Pawn))
  ;[1 1 1] Permet au vaisseau de se déplacer
  (Pawn|Input|AddMovementInput (Math|Vector|GetForwardVector (Math|Rotator|MakeRotator 0.0 0.0 (.yaw _returnvalue))) (.y ActionValue) false)
  (Pawn|Input|AddMovementInput (Math|Vector|GetRightVector (Math|Rotator|MakeRotator 0.0 0.0 (.yaw _returnvalue))) (.x ActionValue) false))

(event Input|EnhancedActionEvents|EnhancedInputActionINP_Fire
  (params (ActionValue :type Boolean) (ElapsedSeconds :type Float%20%28double-precision%29) (TriggeredSeconds :type Float%20%28double-precision%29) (InputAction :type Input%20Action%20Object%20Reference :default "/Game/System/Inputs/INP_Fire.INP_Fire"))
  (bind _projectilespawnpoint (Variables|Default|GetProjectileSpawnPoint))
  (bind _returnvalue (Transformation|GetWorldTransform _projectilespawnpoint))
  ;[1 1 1] Permet au vaisseau de tirer
  (if (Variables|Default|GetcanShoot)
    (Game|SpawnActorfromClass "/Game/Blueprints/BP_Laser.BP_Laser_C" (Math|Transform|MakeTransform (.location _returnvalue) (.rotation _returnvalue) "1.000000,1.000000,1.000000") "Undefined" "MultiplyWithRoot" 0 0)
    (Variables|Default|SetcanShoot false)
    (CallFunction|Reload)))

(event EventBeginPlay
  (bind _returnvalue (Game|GetPlayerController 0))
  (bind _returnvalue_2 (PlayerController|LocalPlayerSubsystems|GetEnhancedInputLocalPlayerSubsystem _returnvalue))
  ;[1 1 1] Initialise les controles
  (Utilities|IsValid _returnvalue_2
    (:Is%20Valid
      (Input|AddMappingContext _returnvalue_2 "/Game/System/Inputs/IMC_Spaceship.IMC_Spaceship" 0 "(bIgnoreAllPressedKeysUntilRelease=True,bForceImmediately=False,bNotifyUserSettings=False)"))))

(fn ConstructionScript)